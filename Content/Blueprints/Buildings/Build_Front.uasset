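; Build_Front is a destructible building front that releases missing-in-action drones when its wall meshes fracture.
; BeginPlay gathers four spawn points and binds the wall fracture events to a one-shot handler.
; That handler plays an explosion, spawns a random number of drones at random points up to the game mode's map limit, and updates the required rescue count.
; The wall pieces then simulate physics, lose collision and are destroyed after delays.
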(event Custom|BindOnCompFracture
  (params (HitPoint :type Vector%20%28by%20ref%29) (HitDirection :type Vector%20%28by%20ref%29))
  (bind _returnvalue (Game|GetGameMode))
  (bind _sm_wall_12_dm1 (Variables|Default|GetSM_Wall_12_DM1))
  (bind _asbp_game_mode_base (Utilities|Casting|CastToBP_GameModeBase _returnvalue))
  (bind _returnvalue_2 (Class|TankGameModeBase|GetMaxMissinginMap _asbp_game_mode_base))
  (Utilities|FlowControl|DoOnce false
    (:Completed
      (Effects|SpawnEmitteratLocation "/Game/CSC/Demo/Particles/P_Explosion.P_Explosion" HitPoint (Math|Rotator|MakeRotfromX HitDirection)) ; ya lo e,iteen los mesh
      ;[1 1 1] Poner esta funci'on en el game mode
      (Variables|Default|SetNumberMissingInCombat (/ _returnvalue_2 10))
      ;;[1 1 1] Spawn Drones
      (for _index (range 0 (Math|Random|RandomIntegerinRange (Variables|Default|GetNumberMinOfMissingToSpawn) _returnvalue_2))
        (Utilities|SpawnMissing _returnvalue_2))
      (bind _asbp_game_mode_base_2 (Utilities|Casting|CastToBP_GameModeBase (Game|GetGameMode)))
      (Class|TankGameModeBase|SetMissingRequired _asbp_game_mode_base_2) ; Aquí memorizamos los drones engendrados par<a saber cuántos tenemos que salvar por nivel
      (Physics|SetSimulatePhysics (Variables|Default|GetSM_Wall_12_DM) true)
      (Utilities|FlowControl|Delay 3.0)
      (Physics|SetSimulatePhysics _sm_wall_12_dm1 false)
      (Collision|SetCollisionEnabled _sm_wall_12_dm1 "NoCollision")
      (Utilities|FlowControl|Delay 5.0)
      (Components|DestroyComponent (Variables|Default|GetSM_Wall_12_DM)))))

(event EventBeginPlay
  (bind _spawnpoints (Variables|Default|GetSpawnPoints))
  (Utilities|FlowControl|Sequence
    (:then_0
      (Utilities|Array|Add _spawnpoints (Variables|Default|GetSpawnPoint))
      (Utilities|Array|Add _spawnpoints (Variables|Default|GetSpawnPoint1))
      (Utilities|Array|Add _spawnpoints (Variables|Default|GetSpawnPoint2))
      (Utilities|Array|Add _spawnpoints (Variables|Default|GetSpawnPoint3)))
    (:then_2
      (EventDispatchers|BindEventtoOnComponentFracture (Variables|Default|GetSM_Wall_12_DM) (delegate Custom|BindOnCompFracture)))))

(fn ConstructionScript)