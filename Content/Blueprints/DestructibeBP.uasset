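; Destructible wall Blueprint that releases AI pawns the first time one of its pieces breaks.
; BeginPlay binds four destructible wall components to one fracture handler, gated by DoOnce.
; The handler plays steam at the hit point, then spawns two TestPNJ and two PNJ pawns at four directional arrows.
; A randomized SpawnLocation is computed at BeginPlay but the spawns ignore it, and several leftover nodes are disconnected.
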(event Custom|BindOnCompFracture
  (params (HitPoint :type Vector%20%28by%20ref%29) (HitDirection :type Vector%20%28by%20ref%29))
  (Utilities|FlowControl|DoOnce false
    (:Completed
      (Effects|SpawnEmitteratLocation "/Game/StarterContent/Particles/P_Steam_Lit.P_Steam_Lit" HitPoint (Math|Rotator|MakeRotfromX HitDirection))
      (Utilities|FlowControl|Sequence
        (:then_0
          (AI|SpawnAIFromClass "/Game/Blueprints/PNJ/TestPNJ.TestPNJ_C" 0 (Transformation|GetWorldLocation (Variables|Default|GetArrowRight)) "0, 0, 0" false (AI|GetAIController 0)))
        (:then_1
          (AI|SpawnAIFromClass "/Game/Blueprints/PNJ/TestPNJ.TestPNJ_C" 0 (Transformation|GetWorldLocation (Variables|Default|GetArrowFront)) "0, 0, 0" false (AI|GetAIController 0)))
        (:then_2
          (AI|SpawnAIFromClass "/Game/Blueprints/PNJ.PNJ_C" 0 (Transformation|GetWorldLocation (Variables|Default|GetArrowLeft)) "0, 0, 0" false (AI|GetAIController 0)))
        (:then_3
          (AI|SpawnAIFromClass "/Game/Blueprints/PNJ.PNJ_C" 0 (Transformation|GetWorldLocation (Variables|Default|GetArrowBack)) "0, 0, 0" false (AI|GetAIController 0)))))))

(event Custom|FindLocToSPawn
  (bind _arrowright (Variables|Default|GetArrowRight))
  (bind _arrowfront (Variables|Default|GetArrowFront))
  (bind _returnvalue (Transformation|GetWorldLocation _arrowfront))
  (bind _returnvalue_2 (Transformation|GetWorldLocation _arrowright))
  (Utilities|FlowControl|FlipFlop
    (:A
      (Variables|Default|SetSpawnLocation (Math|Vector|MakeVector (.x _returnvalue_2) (+ (Math|Random|RandomFloatinRange 1e+03 2e+03) (.y _returnvalue_2)) (.z _returnvalue_2))))
    (:B
      (Variables|Default|SetSpawnLocation (Math|Vector|MakeVector (+ (.x _returnvalue) (Math|Random|RandomFloatinRange -1e+03 -2e+03)) (.y _returnvalue) (.z _returnvalue))))))

(event EventBeginPlay
  (Utilities|FlowControl|Sequence
    (:then_0
      (CallFunction|FindLoctoSPawn))
    (:then_1
      (EventDispatchers|BindEventtoOnComponentFracture (Variables|Default|GetSM_Wall_Down_TubesQuard_Orange_DM) (delegate Custom|BindOnCompFracture)))))

(fn ConstructionScript)