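; Destructible camp that releases missing-in-action drones for the player to rescue when its walls are broken.
; The first fracture of any of four destructible wall components triggers a one-time spawn of a few drones at random picks from four arrow points.
; A macro caps live drones level-wide, and each spawn updates the game mode's required rescue count.
; Several older spawn and location experiments remain unwired.
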(event Custom|BindOnCompFracture
  (params (HitPoint :type Vector%20%28by%20ref%29) (HitDirection :type Vector%20%28by%20ref%29))
  (Utilities|FlowControl|DoOnce false
    (:Completed
      (Variables|Default|SetNumberMissingInCombat 25) ; Limitar un numero máximo para evitar bugs
      (for _index (range 0 (Math|Random|RandomIntegerinRange 2 4))
        (Utilities|SpawnMissing (Variables|Default|GetNumberMissingInCombat))
        (bind _asbp_game_mode_base (Utilities|Casting|CastToBP_GameModeBase (Game|GetGameMode)))
        (Class|TankGameModeBase|SetMissingRequired _asbp_game_mode_base) ; Aquí memorizamos los drones engendrados par<a saber cuántos tenemos que salvar por nivel
      ))))

(event Custom|FindLocToSPawn
  (bind _arrowright (Variables|Default|GetArrowRight))
  (bind _arrowfront (Variables|Default|GetArrowFront))
  (bind _returnvalue (Transformation|GetWorldLocation _arrowfront))
  (bind _returnvalue_2 (Transformation|GetWorldLocation _arrowright))
  (Utilities|FlowControl|FlipFlop
    (:A
      (Variables|Default|SetSpawnLocation (Math|Vector|MakeVector (.x _returnvalue_2) (+ (Math|Random|RandomFloatinRange 1e+03 2e+03) (.y _returnvalue_2)) (.z _returnvalue_2))))
    (:B
      (Variables|Default|SetSpawnLocation (Math|Vector|MakeVector (+ (.x _returnvalue) (Math|Random|RandomFloatinRange -1e+03 -2e+03)) (.y _returnvalue) (.z _returnvalue))))))

(event EventBeginPlay
  (Utilities|FlowControl|Sequence
    (:then_0
      (Utilities|Array|Insert (Variables|Default|GetPointsToSpawnsArray) (Variables|Default|GetArrowRight))
      (Utilities|Array|Insert (Variables|Default|GetPointsToSpawnsArray) (Variables|Default|GetArrowFront) 1)
      (Utilities|Array|Insert (Variables|Default|GetPointsToSpawnsArray) (Variables|Default|GetArrowLeft) 2)
      (Utilities|Array|Insert (Variables|Default|GetPointsToSpawnsArray) (Variables|Default|GetArrowBack) 3))
    (:then_1
      (EventDispatchers|BindEventtoOnComponentFracture (Variables|Default|GetSM_Wall_Down_TubesQuard_Orange_DM) (delegate Custom|BindOnCompFracture)))))

(fn ConstructionScript)