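; Game instance for a tank game that handles local saves, gold coins and in-app purchase state.
; Progress saves store player transform, missing-in-action, score and level, with load, respawn and new-game wipe.
; Coin and tank-purchase saves each write a fresh object to one shared slot, overwriting each other's fields.
; IAP support is partial: unprocessed receipts unlock only Panther, restore just lists product IDs, and SaveLevel never writes to disk.
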(event Custom|SaveGame
  (bind _returnvalue (Game|Player|GetPlayerPawn 0))
  (bind _aspt_pawn_hero (Utilities|Casting|CastToPT_PawnHero _returnvalue))
  ;[1 1 1] Save Games / version sin IAPurchased en codigo Y sólo almacenamos levelID y Score; si empiza partida se empieza de nuevo
  (bind _returnvalue_2 (SaveGame|CreateSaveGameObject "/Game/Blueprints/GameInstance/BP_SaveGame.BP_SaveGame_C"))
  (Variables|/Game/Blueprints/GameInstance/BP_SaveGame.BP_SaveGame_C|SetPawnLocation _returnvalue_2 (Transformation|GetActorLocation _aspt_pawn_hero))
  (Variables|/Game/Blueprints/GameInstance/BP_SaveGame.BP_SaveGame_C|SetTranform_Player _returnvalue_2 (Transformation|GetWorldTransform (Variables|/Script/ToonTanks.PawnBase|GetCapsuleComp _aspt_pawn_hero)))
  (Variables|/Game/Blueprints/GameInstance/BP_SaveGame.BP_SaveGame_C|SetMissingInActions _returnvalue_2 (Class|PawnTank|GetMissinginAction _aspt_pawn_hero))
  (Variables|/Game/Blueprints/GameInstance/BP_SaveGame.BP_SaveGame_C|SetScore _returnvalue_2 (Class|TankGameModeBase|GetScore (.AsTank%20Game%20Mode%20Base (Utilities|Casting|CastToTankGameModeBase (Game|GetGameMode)))))
  (bind _returnvalue_3 (Game|GetCurrentLevelName true))
  (Variables|/Game/Blueprints/GameInstance/BP_SaveGame.BP_SaveGame_C|SetLevelName _returnvalue_2 (Utilities|String|StringToName _returnvalue_3))
  (SaveGame|SaveGametoSlot _returnvalue_2 (Variables|Default|GetSaveGameSettings))
  (Development|PrintString "Save game"))

(event Custom|loadGame
  (bind _savegamesettings (Variables|Default|GetSaveGameSettings))
  ;[1 1 1] Load games  / deprected en código, y sólo almacenaos Score y LevelID,
  (bind _returnvalue (SaveGame|DoesSaveGameExist _savegamesettings))
  (if _returnvalue
    (bind _returnvalue_2 (SaveGame|LoadGamefromSlot _savegamesettings))
    (bind _asbp_save_game (Utilities|Casting|CastToBP_SaveGame _returnvalue_2))
    (Utilities|FlowControl|Sequence
      (:then_0
        (bind _returnvalue_3 (Game|GetCurrentLevelName true))
        (if (not (Utilities|Enum|Equal(Enum) _returnvalue_3 (Utilities|String|ToString(Name) (Variables|/Game/Blueprints/GameInstance/BP_SaveGame.BP_SaveGame_C|GetLevelName _asbp_save_game))))
          (Game|OpenLevel(byName) (Variables|/Game/Blueprints/GameInstance/BP_SaveGame.BP_SaveGame_C|GetLevelName _asbp_save_game))))
      (:then_1
        (Utilities|FlowControl|Delay 0.2)
        (bind _aspt_pawn_hero (Utilities|Casting|CastToPT_PawnHero (Game|Player|GetPlayerPawn 0)))
        (Class|PawnTank|SetMissinginAction _aspt_pawn_hero (Variables|/Game/Blueprints/GameInstance/BP_SaveGame.BP_SaveGame_C|GetMissingInActions _asbp_save_game))
        (Transformation|SetActorTransform _aspt_pawn_hero (Math|Transform|MakeTransform (Variables|/Game/Blueprints/GameInstance/BP_SaveGame.BP_SaveGame_C|GetPawnLocation _asbp_save_game) (.rotation (Variables|/Game/Blueprints/GameInstance/BP_SaveGame.BP_SaveGame_C|GetTranform_Player _asbp_save_game)) "1,1,1") true true)
        (bind _astank_game_mode_base (Utilities|Casting|CastToTankGameModeBase (Game|GetGameMode)))
        (Class|TankGameModeBase|SetScore _astank_game_mode_base (Variables|/Game/Blueprints/GameInstance/BP_SaveGame.BP_SaveGame_C|GetScore _asbp_save_game)))
      (:then_2
        (Development|PrintString "Partida cargada")))
    (else
      (Development|PrintString "Partida Salvada no encontrada: creando partida Salvada")
      (Utilities|FlowControl|Delay 0.2)
      (CallFunction|SaveGame))))

(event Custom|NewGame
  ;[1 1 1] New Game, Overwirte last game
  (bind _returnvalue (SaveGame|DoesSaveGameExist (Variables|Default|GetSaveGameSettings)))
  (if _returnvalue
    (SaveGame|DeleteGameinSlot (Variables|Default|GetSaveGameSettings))))

(event Custom|SaveCoins
  (params (DeltaCoins :type Integer))
  ;[1 1 1] Save vercion con  IAP to Upload  the play game services and retriveing data when Init game
  (CallFunction|SetCoins DeltaCoins)
  (bind _returnvalue (SaveGame|CreateSaveGameObject "/Game/Blueprints/GameInstance/BP_SaveTanksToGameservices.BP_SaveTanksToGameServices_C"))
  (Variables|/Game/Blueprints/GameInstance/BP_SaveTanksToGameservices.BP_SaveTanksToGameServices_C|SetGoldCoins _returnvalue (CallFunction|GetGoldCoins))
  (SaveGame|SaveGametoSlot _returnvalue (Variables|Default|GetSaveTanksSettings))
  (Development|PrintString "Save game"))

(event Custom|SaveLevel
  ;[1 1 1] Save vercion con  IAP to Upload  the play game services and retriveing data when Init game
  (bind _returnvalue (SaveGame|CreateSaveGameObject "/Game/Blueprints/GameInstance/BP_SaveTanksToGameservices.BP_SaveTanksToGameServices_C")))

(event Custom|LoadIAPLocalData
  (bind _savetankssettings (Variables|Default|GetSaveTanksSettings))
  ;[1 1 1] Save vercion con  IAP to Upload  the play game services and retriveing data when Init game
  (bind _returnvalue (SaveGame|DoesSaveGameExist _savetankssettings))
  (if _returnvalue
    (bind _returnvalue_2 (SaveGame|LoadGamefromSlot _savetankssettings))
    (bind _asbp_save_tanks_to_game_services (Utilities|Casting|CastToBP_SaveTanksToGameServices _returnvalue_2))
    (Variables|IAPSettings|SetIAP_Panther_purchased (Variables|/Game/Blueprints/GameInstance/BP_SaveTanksToGameservices.BP_SaveTanksToGameServices_C|GetPantherPurchased _asbp_save_tanks_to_game_services))
    (Variables|IAPSettings|SetIAP_Byshop_purchased (Variables|/Game/Blueprints/GameInstance/BP_SaveTanksToGameservices.BP_SaveTanksToGameServices_C|GetByshopPurchased _asbp_save_tanks_to_game_services))
    (Variables|IAPSettings|SetIAP_Tyger_purchased (Variables|/Game/Blueprints/GameInstance/BP_SaveTanksToGameservices.BP_SaveTanksToGameServices_C|GetTygerPurchased _asbp_save_tanks_to_game_services))
    (Variables|IAPSettings|SetIAP_Levels_purchased_ (Variables|/Game/Blueprints/GameInstance/BP_SaveTanksToGameservices.BP_SaveTanksToGameServices_C|GetLevelsPruchased _asbp_save_tanks_to_game_services))))

(event Custom|SpawnAgain
  (bind _savegamesettings (Variables|Default|GetSaveGameSettings))
  (bind _returnvalue (SaveGame|DoesSaveGameExist _savegamesettings))
  (if _returnvalue
    (bind _returnvalue_2 (SaveGame|LoadGamefromSlot _savegamesettings))
    (bind _asbp_save_game (Utilities|Casting|CastToBP_SaveGame _returnvalue_2))
    (bind _aspt_pawn_hero (Utilities|Casting|CastToPT_PawnHero (Game|Player|GetPlayerPawn 0)))
    (Class|Actor|AddActorLocalTransform _aspt_pawn_hero (Variables|/Game/Blueprints/GameInstance/BP_SaveGame.BP_SaveGame_C|GetTranform_Player _asbp_save_game) true true)
    (else
      (Development|PrintString "Partida Salvada no encontrada: creando partida Salvada")
      (Utilities|FlowControl|Delay 0.2)
      (CallFunction|SaveGame))))

(event Custom|RestoringPurchases
  (bind _iap_prodid (Variables|Default|GetIAP_ProdID))
  (Utilities|Array|AddUnique _iap_prodid (Variables|IAPSettings|GetIAP_panthertank))
  (Utilities|Array|AddUnique _iap_prodid (Variables|IAPSettings|GetIAP_byshoptank))
  (Utilities|Array|AddUnique _iap_prodid (Variables|IAPSettings|GetIAP_tygertanks))
  (Utilities|Array|AddUnique _iap_prodid (Variables|IAPSettings|GetIAP_removeads)))

(event Custom|UpdateTanks
  (Development|PrintString "OnUnexpectedPurchase" true true "(R=1.000000,G=0.000000,B=0.031557,A=1.000000)" 1e+01)
  (bind _inapppurchasereceipts (|InAppPurchaseUnprocessed2 (Game|GetPlayerController 0)) ; Te retorna todos los productos
    (:OnSuccess
      (for _array_element _inapppurchasereceipts
        (if (Utilities|Enum|Equal(Enum) (.ItemName (Utilities|Struct|BreakInAppPurchaseReceiptInfo2 _array_element)) (Variables|IAPSettings|GetIAP_panthertank))
          (CallFunction|SetPantherTankPurchase)))
      (Variables|Default|SetIdprod 0))))

(event Custom|HandleGoldPurchase
  ;[1 1 1] Save in local  Tanks purchased
)

(event Custom|SaveTankPurchase
  ;[1 1 1] Save in local  Tanks purchased
  (bind _returnvalue (SaveGame|CreateSaveGameObject "/Game/Blueprints/GameInstance/BP_SaveTanksToGameservices.BP_SaveTanksToGameServices_C"))
  (Variables|/Game/Blueprints/GameInstance/BP_SaveTanksToGameservices.BP_SaveTanksToGameServices_C|SetTygerPurchased _returnvalue (Variables|IAPSettings|GetIAP_Tyger_purchased))
  (Variables|/Game/Blueprints/GameInstance/BP_SaveTanksToGameservices.BP_SaveTanksToGameServices_C|SetByshopPurchased _returnvalue (Variables|IAPSettings|GetIAP_Byshop_purchased))
  (Variables|/Game/Blueprints/GameInstance/BP_SaveTanksToGameservices.BP_SaveTanksToGameServices_C|SetPantherPurchased _returnvalue (Variables|IAPSettings|GetIAP_Panther_purchased))
  (SaveGame|SaveGametoSlot _returnvalue (Variables|Default|GetSaveTanksSettings))
  (Development|PrintString "Save game"))

(event Custom|CheckIsPantherPurchased
  (Development|PrintString "OnUnexpectedPurchase" true true "(R=1.000000,G=0.000000,B=0.031557,A=1.000000)" 1e+01)
  (bind _inapppurchasereceipts (|InAppPurchaseUnprocessed2 (Game|GetPlayerController 0)) ; Te retorna todos los productos
    (:OnSuccess
      (for _array_element _inapppurchasereceipts
        (if (Utilities|Enum|Equal(Enum) (.ItemName (Utilities|Struct|BreakInAppPurchaseReceiptInfo2 _array_element)) (Variables|IAPSettings|GetIAP_panthertank))
          (CallFunction|SetPantherTankPurchase)))
      (Variables|Default|SetIdprod 0))))

(event EventInit
  ;[1 1 1] Save in local  Tanks purchased
)

(fn GetIsSavedGame
  (bind _returnvalue (SaveGame|DoesSaveGameExist (Variables|Default|GetSaveGameSettings)))
  (return _returnvalue))

(fn HandlePurchasesSucces
  (params (DeltaCoins :type Integer) (CallingWidget :type WB%20Store%20Object%20Reference))
  (bind _returnvalue (Utilities|IsValid CallingWidget))
  (Development|PrintString "*** Saving Purchase Locally ***")
  (if (<= DeltaCoins 0)
    (CallFunction|SaveLevel)
    (if _returnvalue
      (Default|UpdateUILevel CallingWidget)
      (else
        (Development|PrintString "--- Handle Theme Not Called From A Widget ---" :!label _label)))
    (else
      (CallFunction|SaveCoins DeltaCoins)
      (if _returnvalue
        (Default|UpdateUI CallingWidget :!pinned true) ; indicar si qué set
        (else
          (goto _label))))))

(fn GetGoldCoins
  (return (Variables|Default|GetCoins)))

(fn SetCoins
  (params (DeltaCoins :type Integer))
  (Variables|Default|SetCoins (+ DeltaCoins (Variables|Default|GetCoins))))

(fn SetPantherTankPurchase
  (Variables|IAPSettings|SetIAP_Panther_purchased true)
  (CallFunction|SaveTankPurchase))

(fn GetTygerTanksPurchased
  (return (Variables|IAPSettings|GetIAP_Tyger_purchased)))

(fn GetPantherTanksPurchased
  (return (Variables|IAPSettings|GetIAP_Panther_purchased)))

(fn GetByshopTanksPurchased
  (return (Variables|IAPSettings|GetIAP_Byshop_purchased)))

(fn SetByshopTankPurchase
  (Variables|IAPSettings|SetIAP_Byshop_purchased true)
  (CallFunction|SaveTankPurchase))

(fn SetTygerTankPurchase
  (Variables|IAPSettings|SetIAP_Tyger_purchased true)
  (CallFunction|SaveTankPurchase))

(fn SetRemoveAdsPurchase
  (Variables|IAPSettings|SetIAP_RemovesAd_purchased true)
  (CallFunction|SaveTankPurchase))