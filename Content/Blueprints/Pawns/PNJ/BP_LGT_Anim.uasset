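; Animated LGT tank actor in the NPC pawns folder that acts as a pickup for the hero pawn, with the upgrade only a debug print.
; Tick scrolls the track texture by feeding game time into a material parameter, creating the dynamic material instance every frame.
; When PT_PawnHero overlaps the sphere, it prints "Upgrade tank", spawns an explosion and destroys itself after a short delay.
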(event OnComponentBeginOverlap(Sphere)
  (params (OverlappedComponent :type Primitive%20Component%20Object%20Reference) (OtherActor :type Actor%20Object%20Reference) (OtherComp :type Primitive%20Component%20Object%20Reference) (OtherBodyIndex :type Integer) (bFromSweep :type Boolean) (SweepResult :type Hit%20Result%20Structure%20%28by%20ref%29))
  (Utilities|Casting|CastToPT_PawnHero OtherActor)
  (Development|PrintString "Upgrade tank")
  (Effects|SpawnEmitteratLocation "/Game/Assets/EpicContent/Particles/P_Explosion.P_Explosion" "0, 0, 0")
  (Utilities|FlowControl|Delay 0.2)
  (Actor|DestroyActor))

(event EventBeginPlay)

(event Collision|EventActorBeginOverlap
  (params (OtherActor :type Actor%20Object%20Reference)))

(event EventTick
  (params (DeltaSeconds :type Float%20%28single-precision%29))
  (bind _returnvalue (Rendering|Material|CreateDynamicMaterialInstance (Variables|SkeletalMeshActor|GetSkeletalMeshComponent) 1 "/Game/Assets/CSC/Materials/M_LGT_Tracks.M_LGT_Tracks" "None" :!class /Script/Engine.PrimitiveComponent))
  (bind _output_get (Variables|Default|SetMatInstance _returnvalue))
  (Rendering|Material|SetScalarParameterValue _output_get "V_texCoord" (/ (Utilities|Time|GetTimeSeconds) 1.0) :!class /Script/Engine.MaterialInstanceDynamic))

(fn ConstructionScript)