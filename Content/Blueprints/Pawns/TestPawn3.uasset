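; Test pawn that turns toward and follows the player's PT_PawnHero, halting once it is closer than 750 units.
; Each Tick, CheckDistance gates RotateBase, which yaws the mesh at the player's height-flattened location and returns that rotation.
; The root moves one unit per frame along it, without sweep or delta-time scaling.
; RutePoint actors are cached at BeginPlay, but MoveForward, which targets the first, is never called.
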(event EventBeginPlay
  (Utilities|FlowControl|Sequence
    (:then_0
      (bind _outactors (Actor|GetAllActorsOfClass "/Game/Blueprints/RutePoint.RutePoint_C"))
      (Variables|Default|SetRutePointsArray _outactors))))

(event EventTick
  (params (DeltaSeconds :type Float%20%28single-precision%29))
  (bind _returnvalue (Game|Player|GetPlayerPawn 0))
  (bind _aspt_pawn_hero (Utilities|Casting|CastToPT_PawnHero _returnvalue))
  (bind _bigogomove (CallFunction|CheckDistance _aspt_pawn_hero 7.5e+02))
  (if _bigogomove
    (bind _rotatormesh (CallFunction|RotateBase (Transformation|GetWorldLocation (Variables|/Script/Engine.Actor|GetRootComponent _returnvalue))))
    (Transformation|AddWorldOffset (Variables|Default|GetDefaultSceneRoot) (Math|Vector|GetForwardVector _rotatormesh) false false)
    (else
      (Development|PrintString "stop"))))

(fn ConstructionScript)

(fn CheckDistance
  (params (PawnPlayer :type Actor%20Object%20Reference) (DistanceMinToAttack :type Float%20%28single-precision%29))
  (if (>= (Transformation|GetDistanceTo PawnPlayer self) DistanceMinToAttack)
    (return true)
    (else
      (return false))))

(fn CheckDistance0
  (params (PawnPlayer :type Actor%20Object%20Reference) (DistanceMinToAttack :type Float%20%28single-precision%29))
  (if (>= (Transformation|GetDistanceTo PawnPlayer self) DistanceMinToAttack)
    (return true)
    (else
      (return false))))

(fn MoveForward
  (params (Value :type Float%20%28single-precision%29))
  (bind _rotatormesh (CallFunction|RotateBase (Transformation|GetWorldLocation (Variables|/Game/Blueprints/RutePoint.RutePoint_C|GetBillboard (Utilities|Array|Get(acopy) (Variables|Default|GetRutePointsArray))))))
  (Variables|Default|SetVelocity (* (* (Math|Vector|GetForwardVector _rotatormesh) 2e+01) Value)))

(fn RotateBase
  (params (LookAtTarget :type Vector))
  (bind _staticmesh (Variables|Default|GetStaticMesh))
  (bind _staticmesh_2 (Variables|Default|GetStaticMesh))
  (bind _returnvalue (Transformation|GetWorldLocation _staticmesh))
  (bind _returnvalue_2 (Transformation|GetWorldLocation _staticmesh_2))
  (bind _returnvalue_3 (Math|Rotator|FindLookatRotation _returnvalue_2 (Math|Vector|MakeVector (.x LookAtTarget) (.y LookAtTarget) (.z _returnvalue))))
  (Transformation|SetWorldRotation (Variables|Default|GetStaticMesh) _returnvalue_3 false false)
  (return _returnvalue_3))

(fn NewFunction0)