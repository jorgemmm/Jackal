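; Enemy tank pawn Blueprint that adds an overhead info widget and damage text feedback on top of its parent class.
; Each Tick copies health into the widget's bar, turns it toward the player while the hero is alive, and hides it beyond a 2D distance threshold.
; AnyDamage spawns a damage text component at the tank's transform, throttled by a DoOnce that resets after a short delay.
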(event EventBeginPlay)

(event Collision|EventActorBeginOverlap
  (params (OtherActor :type Actor%20Object%20Reference)))

(event EventTick
  (params (DeltaSeconds :type Float%20%28single-precision%29))
  (bind _returnvalue (Game|Player|GetPlayerPawn 0))
  (bind _infowbp (Variables|Default|GetInfoWBP))
  (bind _healthcomponent (Variables|Default|GetHealthComponent))
  (bind _infowbp_2 (Variables|Default|GetInfoWBP))
  (bind _aspt_pawn_hero (Utilities|Casting|CastToPT_PawnHero _returnvalue))
  (|CallParentFunction DeltaSeconds)
  (Utilities|FlowControl|Sequence
    (:then_0
      (bind _aswbp_hulk_points (Utilities|Casting|CastToWBP_HulkPoints (UserInterface|GetUserWidgetObject (Variables|Default|GetInfoWBP))))
      (Progress|SetPercent (Variables|/Game/Blueprints/Widgets/WBP_HulkPoints.WBP_HulkPoints_C|GetHuklPointsBar _aswbp_hulk_points) (/ (Class|HealthComponent|GetHealth _healthcomponent) (Variables|/Script/ToonTanks.HealthComponent|GetDefaultHealth _healthcomponent))))
    (:then_1
      ;[1 1 1] Rota info bar to player pawn if damage
      (if (> (Class|HealthComponent|GetHealth (Variables|/Script/ToonTanks.PawnBase|GetHealthComponent _aspt_pawn_hero)) 0.0)
        (Transformation|SetWorldRotation _infowbp_2 (Math|Rotator|FindLookatRotation (Transformation|GetWorldLocation _infowbp_2) (Transformation|GetActorLocation _aspt_pawn_hero)) false false)))
    (:then_3
      (if (>= (Math|Vector|Distance2D(Vector) (Transformation|GetActorLocation (.AsPT%20Pawn%20Hero (Utilities|Casting|CastToPT_PawnHero (Game|Player|GetPlayerPawn 0)))) (Transformation|GetActorLocation)) (Variables|Default|GetUmbralDistRendim))
        (Rendering|SetVisibility _infowbp false false)
        (else
          (Rendering|SetVisibility _infowbp true false))))))

(event Game|Damage|EventRadialDamage
  (params (DamageReceived :type Float%20%28single-precision%29) (DamageType :type Damage%20Type%20Object%20Reference) (Origin :type Vector :default "0, 0, 0") (HitInfo :type Hit%20Result%20Structure%20%28by%20ref%29) (InstigatedBy :type Controller%20Object%20Reference) (DamageCauser :type Actor%20Object%20Reference)))

(event Game|Damage|EventAnyDamage
  (params (Damage :type Float%20%28single-precision%29) (DamageType :type Damage%20Type%20Object%20Reference) (InstigatedBy :type Controller%20Object%20Reference) (DamageCauser :type Actor%20Object%20Reference))
  (Utilities|FlowControl|DoOnce false :!label _label
    (:Completed
      (bind _returnvalue (AddComponent|AddWCDamageText true (Transformation|GetActorTransform)))
      (Default|SetDamageText _returnvalue Damage)
      (Utilities|FlowControl|Delay 2.0)
      (goto _label Reset))))

(fn ConstructionScript)