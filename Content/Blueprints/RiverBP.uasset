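; RiverBP is a river or hole hazard actor built around a box collision that detects the hero tank pawn.
; A box hit stores the PT_PawnHero as TankHero and prints a warning.
; LevelDamage applies fixed damage to the stored tank, but nothing live calls it.
; The timer start and clear logic is disconnected, and the overlap events are empty, so the hazard currently only warns.
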(event OnComponentBeginOverlap(Box)
  (params (OverlappedComponent :type Primitive%20Component%20Object%20Reference) (OtherActor :type Actor%20Object%20Reference) (OtherComp :type Primitive%20Component%20Object%20Reference) (OtherBodyIndex :type Integer) (bFromSweep :type Boolean) (SweepResult :type Hit%20Result%20Structure%20%28by%20ref%29)))

(event OnComponentEndOverlap(Box)
  (params (OverlappedComponent :type Primitive%20Component%20Object%20Reference) (OtherActor :type Actor%20Object%20Reference) (OtherComp :type Primitive%20Component%20Object%20Reference) (OtherBodyIndex :type Integer)))

(event OnComponentHit(Box)
  (params (HitComponent :type Primitive%20Component%20Object%20Reference) (OtherActor :type Actor%20Object%20Reference) (OtherComp :type Primitive%20Component%20Object%20Reference) (NormalImpulse :type Vector :default "0, 0, 0") (Hit :type Hit%20Result%20Structure%20%28by%20ref%29))
  (bind _aspt_pawn_hero (Utilities|Casting|CastToPT_PawnHero OtherActor))
  (Variables|Default|SetTankHero _aspt_pawn_hero)
  (Development|PrintString "Warning with River or Hole"))

(event Custom|LevelDamage
  (Utilities|IsValid (Variables|Default|GetTankHero)
    (:Is%20Valid
      (Game|Damage|ApplyDamage (Variables|Default|GetTankHero) 25.0 (Game|GetInstigatorController) self "/Script/Engine.DamageType"))
    (:Is%20Not%20Valid
      (Development|PrintString "No tank detected"))))

(event EventBeginPlay)

(event Collision|EventActorBeginOverlap
  (params (OtherActor :type Actor%20Object%20Reference)))

(event EventTick
  (params (DeltaSeconds :type Float%20%28single-precision%29)))

(fn ConstructionScript)