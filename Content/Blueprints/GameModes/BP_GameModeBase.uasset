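; Base game mode for a tank game that manages start and end screens, the HUD and music.
; GameStart shows the start widget and adds the HUD after a delay, while GameOver swaps the HUD for a win/lose screen.
; A delayed Tick polls hero health, using paired DoOnce gates to switch between gameplay and game-over music.
; UpdateTank replaces the player's pawn with a Panther at the same transform and possesses it.
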(event EventBeginPlay)

(event EventTick
  (params (DeltaSeconds :type Float%20%28single-precision%29))
  (Utilities|FlowControl|Delay 1.0)
  (bind _aspt_pawn_hero (Utilities|Casting|CastToPT_PawnHero (Game|Player|GetPlayerPawn 0)))
  (if (<= (Class|HealthComponent|GetHealth (Variables|/Script/ToonTanks.PawnBase|GetHealthComponent _aspt_pawn_hero)) 0.0)
    (Utilities|FlowControl|DoOnce false :!label _label
      (:Completed
        (if (!= (Variables|Default|GetArcademusic3) 0)
          (Audio|Components|Audio|Stop (Variables|Default|GetArcademusic3)))
        (bind _returnvalue (Audio|SpawnSound2D "/Game/Assets/Audio/Music/MegaGameCollection/Funny/CasualArcadeGameOverLoop_Cue.CasualArcadeGameOverLoop_Cue" 1.0 1.0 0.0 0))
        (Variables|Default|SetArcadeMusic2 _returnvalue)
        (goto _label_2 Reset)))
    (else
      (Utilities|FlowControl|DoOnce false :!label _label_2
        (:Completed
          (if (!= (Variables|Default|GetArcadeMusic2) 0)
            (Audio|Components|Audio|Stop (Variables|Default|GetArcadeMusic2)))
          (bind _returnvalue_2 (Audio|SpawnSound2D "/Game/Assets/Audio/Music/MegaGameCollection/Funny/Casual_Arcade_Track__3__looped__Cue.Casual_Arcade_Track__3__looped__Cue" 1.0 1.0 0.0 0))
          (Variables|Default|SetArcademusic3 _returnvalue_2)
          (goto _label Reset))))))

(event EventGameOver
  (params (PlayerWon :type Boolean))
  ;[1 1 1] GameOver You Win / You  Lose Play Again
  (Utilities|FlowControl|Sequence
    (:then_0
      (Widget|RemovefromParent (Variables|Default|GetWB_HUDRef)))
    (:then_1
      (bind _returnvalue (UserInterface|CreateWidget "/Game/Blueprints/Widgets/WBP_GameEnd.WBP_GameEnd_C" (.AsBP%20Player%20Controller (Utilities|Casting|CastToBP_PlayerController (Game|GetPlayerController 0)))))
      (Default|SetPlayerWin _returnvalue PlayerWon)
      (UserInterface|Viewport|AddtoViewport _returnvalue 0))))

(event EventGameStart
  (bind _returnvalue (Game|GetPlayerController 0))
  (bind _asbp_player_controller (Utilities|Casting|CastToBP_PlayerController _returnvalue))
  ;[1 1 1] GameOver You Win / You  Lose Play Again
  (Utilities|FlowControl|Sequence
    (:then_0
      (bind _returnvalue_2 (UserInterface|CreateWidget "/Game/Blueprints/Widgets/WBP_GameStart.WBP_GameStart_C" _asbp_player_controller))
      (Default|SetStartDelay _returnvalue_2 (Variables|Default|GetStartDelay))
      (UserInterface|Viewport|AddtoViewport _returnvalue_2 1))
    (:then_1
      (Utilities|FlowControl|Delay 5.0)
      (bind _returnvalue_3 (UserInterface|CreateWidget "/Game/Blueprints/Widgets/WBP_HUD.WBP_HUD_C" _asbp_player_controller))
      (bind _output_get (Variables|Default|SetWB_HUDRef _returnvalue_3))
      (UserInterface|Viewport|AddtoViewport _returnvalue_3 0))))

(fn ConstructionScript)

(fn UpdateTank
  (bind _aspt_pawn_hero (Utilities|Casting|CastToPT_PawnHero (Game|Player|GetPlayerPawn 0)))
  (bind _output_get (Variables|Default|SetHome (Transformation|GetWorldTransform (Variables|/Script/ToonTanks.PawnBase|GetBaseMesh _aspt_pawn_hero))))
  (Actor|DestroyActor _aspt_pawn_hero)
  (bind _returnvalue (Game|SpawnActorfromClass "/Game/Blueprints/Pawns/Players/PT_Hero_Panther.PT_Hero_Panther_C" _output_get "Undefined" self 0))
  (Pawn|Possess (Game|GetPlayerController 0) _returnvalue))